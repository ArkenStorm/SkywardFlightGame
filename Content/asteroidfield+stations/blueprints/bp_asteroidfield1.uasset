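; Procedural asteroid field actor that scatters instanced asteroids in a spherical shell around its origin.
; The construction script loops over AsteroidNumber, adding one instance per pass to each of sixteen hierarchical instanced static mesh components.
; Each instance gets a random direction, distance between minimum and maximum, random rotation, and uniform random scale times a multiplier.
; Randomness is unseeded, and the event graph has no active logic.
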(event `self.HierarchicalInstancedStaticMesh1.OnComponentHit`
  (params (HitComponent :type "PrimitiveComponent Object Reference") (OtherActor :type "Actor Object Reference") (OtherComp :type "PrimitiveComponent Object Reference") (NormalImpulse :type "Vector Structure") (Hit :type "HitResult Structure (by ref)")))

(fn `UserConstructionScript`
  (bind _returnvalue (`KismetMathLibrary.MakeTransform` (* (`KismetMathLibrary.RandomUnitVector`) (`KismetMathLibrary.RandomFloatInRange` (`self.Minimum Distance`) (`self.Maximum Distance`))) (`KismetMathLibrary.RandomRotator` false) (`KismetMathLibrary.Conv_DoubleToVector` (* (`KismetMathLibrary.RandomFloatInRange` (`self.Minimum Scale`) (`self.Maximum Scale`)) (`self.Scale Multiplier`)))))
  (for _ (range (+ (`self.Asteroid Number`) 1))
    (`InstancedStaticMeshComponent.AddInstance` (`self.HierarchicalInstancedStaticMesh1`) _returnvalue)
    (`InstancedStaticMeshComponent.AddInstance` (`self.HierarchicalInstancedStaticMesh2`) _returnvalue)
    (`InstancedStaticMeshComponent.AddInstance` (`self.HierarchicalInstancedStaticMesh3`) _returnvalue)
    (`InstancedStaticMeshComponent.AddInstance` (`self.HierarchicalInstancedStaticMesh4`) _returnvalue)
    (`InstancedStaticMeshComponent.AddInstance` (`self.HierarchicalInstancedStaticMesh5`) _returnvalue)
    (`InstancedStaticMeshComponent.AddInstance` (`self.HierarchicalInstancedStaticMesh6`) _returnvalue)
    (`InstancedStaticMeshComponent.AddInstance` (`self.HierarchicalInstancedStaticMesh7`) _returnvalue)
    (`InstancedStaticMeshComponent.AddInstance` (`self.HierarchicalInstancedStaticMesh8`) _returnvalue)
    (`InstancedStaticMeshComponent.AddInstance` (`self.HierarchicalInstancedStaticMesh9`) _returnvalue)
    (`InstancedStaticMeshComponent.AddInstance` (`self.HierarchicalInstancedStaticMesh10`) _returnvalue)
    (`InstancedStaticMeshComponent.AddInstance` (`self.HierarchicalInstancedStaticMesh11`) _returnvalue)
    (`InstancedStaticMeshComponent.AddInstance` (`self.HierarchicalInstancedStaticMesh12`) _returnvalue)
    (`InstancedStaticMeshComponent.AddInstance` (`self.HierarchicalInstancedStaticMesh13`) _returnvalue)
    (`InstancedStaticMeshComponent.AddInstance` (`self.HierarchicalInstancedStaticMesh14`) _returnvalue)
    (`InstancedStaticMeshComponent.AddInstance` (`self.HierarchicalInstancedStaticMesh15`) _returnvalue)
    (`InstancedStaticMeshComponent.AddInstance` (`self.HierarchicalInstancedStaticMesh16`) _returnvalue)))